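; AI controller Blueprint that runs a behavior tree and tracks a target through AI Perception.
; It starts AIBehaviorTree on BeginPlay.
; On each perception update, a successful sight stimulus writes the sensed actor to the "Target Actor" blackboard key, while lost sight or any non-sight stimulus clears it.
; Debug prints report each outcome.
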(event `self.ReceiveBeginPlay`
  (`self.RunBehaviorTree` "/Game/AI/AIBehaviorTree.AIBehaviorTree")
  (`KismetSystemLibrary.PrintText` "Started Behavior Tree."))

(event `self.AIPerception.OnTargetPerceptionUpdated`
  (params (Actor :type "Actor Object Reference") (Stimulus :type "AIStimulus Structure"))
  (bind _returnvalue (`AIPerceptionSystem.GetSenseClassForStimulus` Stimulus))
  (if (== _returnvalue "/Script/AIModule.AISense_Sight")
    (if (`.bSuccessfullySensed` (break `AIStimulus` Stimulus))
      (`BlackboardComponent.SetValueAsObject` (`AIBlueprintHelperLibrary.GetBlackboard` null) "Target Actor" Actor)
      (`KismetSystemLibrary.PrintText` "Success!")
      (else
        (`KismetSystemLibrary.PrintText` "Not Detected")
        (`BlackboardComponent.SetValueAsObject` (`AIBlueprintHelperLibrary.GetBlackboard` null) "Target Actor" null :!label _label)))
    (else
      (`KismetSystemLibrary.PrintText` "Not Running")
      (goto _label))))

(fn `UserConstructionScript`)