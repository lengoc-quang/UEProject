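; Boss enemy that extends a parent class, setting its own sword radius, combo attack montage and boss flag, and playing a delayed monster sound at spawn.
; Tick branches on level name: outside "Island" the boss regenerates health and, when nearly dead, calls BallExplosion on the player once.
; On "Island", the final level, its death shows a victory message on the player's HUD, plays music, then quits the game.
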(event `self.ReceiveBeginPlay`
  (`parent.ReceiveBeginPlay`)
  (set `self.swordRadius` 170.0)
  (set `self.attackAnim` "/Game/Characters/Mixamo/Animations/Combat/Boss_RM_AttackCombo_Anim_Montage.Boss_RM_AttackCombo_Anim_Montage")
  ;[1 1 1] Set Max Health
  (set `self.maxHealth` (`self.health`))
  (set `self.isBoss?` true)
  (`KismetSystemLibrary.Delay` (`KismetMathLibrary.RandomFloatInRange` 3.0 5.0))
  (`GameplayStatics.PlaySoundAtLocation` "/Game/Audio/Monster.Monster" (`self.K2_GetActorLocation`) (struct) 1.0 1.0 0.0 "/Game/Audio/Footsteps/SA_Stomps.SA_Stomps" null null null))

(event `self.ReceiveTick`
  (params (DeltaSeconds :type "Float (single-precision)"))
  ;[1 1 1] Re-health
  (`parent.ReceiveTick` DeltaSeconds)
  (`|ExecutionSequence`
    (:`then_0`
      (bind _returnvalue (`GameplayStatics.GetCurrentLevelName` true))
      (if (not (`KismetStringLibrary.EqualEqual_StrStr` _returnvalue "Island"))
        (if (< (`self.health`) (`self.maxHealth`))
          (`KismetSystemLibrary.Delay` 0.05)
          (`/Engine/EditorBlueprintResources/StandardMacros.IncrementFloat` (`self.health`)))))
    (:`then_1`
      ;[1 1 1] Player Death Control if Not Final Level
      (bind _returnvalue_2 (`GameplayStatics.GetCurrentLevelName` true))
      (if (not (`KismetStringLibrary.EqualEqual_StrStr` _returnvalue_2 "Island"))
        (if (<= (`self.health`) 15.0)
          (`/Engine/EditorBlueprintResources/StandardMacros.DoOnce` false
            (:`Completed`
              (bind _asbp_third_person_character (cast `/Game/ThirdPerson/Blueprints/BP_ThirdPersonCharacter` (`GameplayStatics.GetPlayerCharacter` 0)))
              (`/Game/ThirdPerson/Blueprints/BP_ThirdPersonCharacter.Ball Explosion` _asbp_third_person_character))))
        (elif (<= (`self.health`) 0.0)
          (`/Engine/EditorBlueprintResources/StandardMacros.DoOnce` false
            (:`Completed`
              (`KismetSystemLibrary.Delay` 2.0)
              (bind _asbp_third_person_character_2 (cast `/Game/ThirdPerson/Blueprints/BP_ThirdPersonCharacter` (`GameplayStatics.GetPlayerCharacter` 0)))
              (bind _hud (`/Game/ThirdPerson/Blueprints/BP_ThirdPersonCharacter.hud` _asbp_third_person_character_2))
              (`TextBlock.SetText` (`/Game/UI/WB_HUD.DimensionText` _hud) "YOU SAVED EVERYONE")
              (`/Game/UI/WB_HUD.Play Dimension Animation` _hud)
              (`GameplayStatics.PlaySound2D` "/Game/Audio/Music/Victory_Music.Victory_Music" 1.0 1.0 0.0 null null)
              (`KismetSystemLibrary.Delay` 7.0)
              (`KismetSystemLibrary.QuitGame` null "Quit"))))))))

(fn `UserConstructionScript`
  (`parent.UserConstructionScript`))