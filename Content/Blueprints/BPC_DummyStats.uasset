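; Health component, named for a dummy, that tracks current health against a maximum and drives an HBar health bar.
; DecreaseHealth subtracts damage, sets the bar percent through a cast of DummyBP and returns whether health is depleted.
; IncreaseHealth adds health and refreshes the bar only when the value exceeds the maximum and gets clamped.
; One tick after BeginPlay it caches its owner as BP_ThirdPersonCharacter, a reference these functions never use.
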(event `self.ReceiveBeginPlay`
  (`KismetSystemLibrary.DelayUntilNextTick`)
  (bind _asbp_third_person_character (cast `/Game/ThirdPerson/Blueprints/BP_ThirdPersonCharacter` (`self.GetOwner`)))
  (set `self.Player Character BP` _asbp_third_person_character))

(fn `Decrease Health`
  (params (Damage :type "Float (double-precision)"))
  (returns (`Dead?` :type Boolean))
  (if (not (<= (`self.Current Health`) 0.0))
    (bind _output_get (set `self.Current Health` (- (`self.Current Health`) Damage)))
    (bind _ashbar (cast `/Game/UI/Stats/HBar` (`self.Dummy BP`)))
    (`ProgressBar.SetPercent` (`/Game/UI/Stats/HBar.Health` _ashbar) (/ _output_get (`self.Max Health`)))
    (if (<= (`self.Current Health`) 0.0)
      _
      (else
        (return false))))
  (return true))

(fn `Get Current Health`
  (returns (`Current Health` :type "Float (double-precision)"))
  (return (`self.Current Health`)))

(fn `Increase Health`
  (params (`Added Health` :type "Float (double-precision)"))
  (set `self.Current Health` (+ (`self.Current Health`) `Added Health`))
  (if (> (`self.Current Health`) (`self.Max Health`))
    (set `self.Current Health` (`self.Max Health`))
    (bind _ashbar (cast `/Game/UI/Stats/HBar` (`self.Dummy BP`)))
    (`ProgressBar.SetPercent` (`/Game/UI/Stats/HBar.Health` _ashbar) (/ (`self.Current Health`) (`self.Max Health`)))))