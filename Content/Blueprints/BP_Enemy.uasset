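; Enemy character, regular or boss, that flags player sightings on its AI blackboard and fights with montage attacks.
; Attack runs a light attack, or randomly light or heavy for bosses, gated by forward sphere traces.
; A looping-timer sword trace deals light damage, while heavy montage notifies trigger stomp damage and camera shake.
; Damage updates a camera-facing health bar and ragdolls at zero health; HitReaction is empty, its knockback logic disconnected.
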(event `self.ReceiveBeginPlay`
  ;[0.05098 0.05098 0.05098] Set Speed
  (set `self.maxSpeed` (`CharacterMovementComponent.MaxWalkSpeed` (`self.CharacterMovement`)))
  ;[0.05098 0.05098 0.05098] Set Max Health
  (set `self.maxHealth` (`self.health`)))

(event `Continue Attacking Calc`
  (bind _returnvalue (`self.K2_GetActorLocation`))
  ;[0.05098 0.05098 0.05098] Continue Attacking Calculation
  (bind (_outhit _returnvalue_2) (`KismetSystemLibrary.SphereTraceSingleForObjects` _returnvalue (+ _returnvalue (* (`KismetMathLibrary.GetForwardVector` (`self.K2_GetActorRotation`)) 100.0)) 70.0 (`|MakeArray` "ObjectTypeQuery3" :!type "EObjectTypeQuery Enum")))
  (if _returnvalue_2
    (cast `/Game/ThirdPerson/Blueprints/BP_ThirdPersonCharacter` (`.HitActor` (`GameplayStatics.BreakHitResult` _outhit))
      (:`CastFailed`
        _)))
  (`AnimInstance.Montage_Stop` (`SkeletalMeshComponent.GetAnimInstance` (`self.Mesh`)) 0.75 "/Game/Characters/Mixamo/Animations/Combat/RM_AttackCombo_Anim_Montage.RM_AttackCombo_Anim_Montage")
  (set `self.attacking?` false))

(event `self.ReceiveTick`
  (params (DeltaSeconds :type "Float (single-precision)"))
  ;[0.05098 0.05098 0.05098] Set Widget Look At Camera & Health UI Percent
  (`SceneComponent.K2_SetWorldRotation` (`self.Arrow1`) (`KismetMathLibrary.FindLookAtRotation` (`self.K2_GetActorLocation`) (`self.K2_GetActorLocation` (`GameplayStatics.GetPlayerCameraManager` 0))) false false)
  (`SceneComponent.K2_SetWorldRotation` (`self.Health Bar`) (`KismetMathLibrary.FindLookAtRotation` (`self.K2_GetActorLocation`) (`self.K2_GetActorLocation` (`GameplayStatics.GetPlayerCameraManager` 0))) false false)
  (bind _aswb_enemy_health_bar (cast `/Game/UI/WB_EnemyHealthBar` (`WidgetComponent.GetWidget` (`self.Health Bar`))))
  (`ProgressBar.SetPercent` (`/Game/UI/WB_EnemyHealthBar.HealthBar` _aswb_enemy_health_bar) (/ (`self.health`) (`self.maxHealth`))))

(event `self.PawnSensing.OnSeePawn`
  (params (Pawn :type "Pawn Object Reference"))
  ;[0.05098 0.05098 0.05098] Sees Player?
  (cast `/Game/ThirdPerson/Blueprints/BP_ThirdPersonCharacter` Pawn)
  (bind _asbp_enemy_controller (cast `/Game/AI/BP_EnemyController` (`AIBlueprintHelperLibrary.GetAIController` self)))
  (`BlackboardComponent.SetValueAsBool` (`AIBlueprintHelperLibrary.GetBlackboard` _asbp_enemy_controller) "seeingPlayer?" true))

(event `Attack`
  ;[0.05098 0.05098 0.05098] Attack System
  (if (`self.isBoss?`)
    (if (`KismetMathLibrary.RandomBool`)
      (`self.Light Attack` 200.0 700.0)
      (else
        (`self.Heavy Attack` 150.0 700.0)))
    (else
      (`self.Light Attack` 70.0 150.0))))

(event `Light Attack`
  (params (Radius :type "Float (single-precision)") (Distance :type "Float (single-precision)"))
  (bind _returnvalue (`self.K2_GetActorLocation`))
  ;[0.05098 0.05098 0.05098] Attack System
  (if (not (`self.attacking?`))
    (set `self.attacking?` true)
    (bind (_outhit _returnvalue_2) (`KismetSystemLibrary.SphereTraceSingleForObjects` :`Start` _returnvalue :`End` (+ _returnvalue (* (`KismetMathLibrary.GetForwardVector` (`self.K2_GetActorRotation`)) Distance)) :`Radius` Radius :`ObjectTypes` (`|MakeArray` "ObjectTypeQuery3" :!type "EObjectTypeQuery Enum") :`DrawTime` 0.7))
    (if _returnvalue_2
      (cast `/Game/ThirdPerson/Blueprints/BP_ThirdPersonCharacter` (`.HitActor` (`GameplayStatics.BreakHitResult` _outhit))
        (:`then`
          (`|PlayMontage` (`self.Mesh`) (`self.attackAnim`)
            (:`then`
              (if (`AnimInstance.Montage_IsPlaying` (`SkeletalMeshComponent.GetAnimInstance` (`self.Mesh`)) "/Game/Characters/Mixamo/Animations/Combat/Zombie_Attack_Montage.Zombie_Attack_Montage")
                (set `CharacterMovementComponent.MaxWalkSpeed` 2.0 (`self.CharacterMovement`))
                (`KismetSystemLibrary.Delay` 0.7)
                (set `CharacterMovementComponent.MaxWalkSpeed` (`self.maxSpeed`) (`self.CharacterMovement`))))
            (:`OnCompleted`
              (set `self.attacking?` false))
            (:`OnNotifyBegin`
              (`self.Continue Attacking Calc`))))
        (:`CastFailed`
          (set `self.attacking?` false :!label _label)))
      (else
        (goto _label)))))

(event `Heavy Attack`
  (params (Radius :type "Float (single-precision)") (Distance :type "Float (single-precision)"))
  (bind _returnvalue (`self.K2_GetActorLocation`))
  (bind _returnvalue_2 (`self.K2_GetActorLocation`))
  (bind _returnvalue_3 (`self.K2_GetActorLocation`))
  ;[0.05098 0.05098 0.05098] Attack System
  (if (not (`self.attacking?`))
    (set `self.attacking?` true)
    (bind (_outhit _returnvalue_4) (`KismetSystemLibrary.SphereTraceSingleForObjects` :`Start` _returnvalue_3 :`End` (+ _returnvalue_3 (* (`KismetMathLibrary.GetForwardVector` (`self.K2_GetActorRotation`)) Distance)) :`Radius` Radius :`ObjectTypes` (`|MakeArray` "ObjectTypeQuery3" :!type "EObjectTypeQuery Enum") :`DrawTime` 0.7))
    (if _returnvalue_4
      (cast `/Game/ThirdPerson/Blueprints/BP_ThirdPersonCharacter` (`.HitActor` (`GameplayStatics.BreakHitResult` _outhit))
        (:`then`
          (`|PlayMontage` (`self.Mesh`) "/Game/Characters/Mixamo/Animations/Combat/Zombie_Attack_Montage.Zombie_Attack_Montage"
            (:`then`
              (set `CharacterMovementComponent.MaxWalkSpeed` 0.0 (`self.CharacterMovement`))
              (`KismetSystemLibrary.Delay` 0.7)
              (set `CharacterMovementComponent.MaxWalkSpeed` (`self.maxSpeed`) (`self.CharacterMovement`)))
            (:`OnCompleted`
              (set `self.attacking?` false))
            (:`OnNotifyBegin`
              (`GameplayStatics.PlaySoundAtLocation` "/Game/Audio/Boss_Hit.Boss_Hit" _returnvalue_2 (struct) 1.0 1.0 0.0 null null null null)
              (`GameplayStatics.PlayWorldCameraShake` "/Game/Blueprints/BP_BossCameraShake.BP_BossCameraShake_C" _returnvalue_2 0.0 10000.0)
              (bind (_outhit_2 _returnvalue_5) (`KismetSystemLibrary.SphereTraceSingleForObjects` :`Start` _returnvalue :`End` (+ _returnvalue (* (`KismetMathLibrary.GetForwardVector` (`self.K2_GetActorRotation`)) 275.0)) :`Radius` 90.0 :`ObjectTypes` (`|MakeArray` "ObjectTypeQuery3" :!type "EObjectTypeQuery Enum") :`DrawTime` 0.7))
              (if _returnvalue_5
                (bind (_bblockinghit _binitialoverlap _time _distance _location _impactpoint _normal _impactnormal _physmat _hitactor) (`GameplayStatics.BreakHitResult` _outhit_2))
                (cast `/Game/ThirdPerson/Blueprints/BP_ThirdPersonCharacter` _hitactor
                  (:`then`
                    (`GameplayStatics.ApplyDamage` _hitactor (`self.heavyAttackDamage`))
                    (`GameplayStatics.PlaySoundAtLocation` "/Game/Audio/Boss_Hit_Stomp.Boss_Hit_Stomp" _location (struct) 1.0 1.0 0.0 "/Game/Audio/Footsteps/SA_Stomps.SA_Stomps" null null null))
                  (:`CastFailed`
                    _)))
              (`NiagaraFunctionLibrary.SpawnSystemAtLocation` "/Game/Niagara/NS_StompHit.NS_StompHit" (`SceneComponent.K2_GetComponentLocation` (`self.HeavyStompNiagaraPos`)) (struct) (1.0 1.0 1.0) true true "AutoRelease"))))
        (:`CastFailed`
          (set `self.attacking?` false :!label _label_2)))
      (else
        (goto _label_2)))))

(event `self.ReceiveAnyDamage`
  (params (Damage :type "Float (single-precision)") (DamageType :type "DamageType Object Reference") (InstigatedBy :type "Controller Object Reference") (DamageCauser :type "Actor Object Reference"))
  ;[0.05127 0.05127 0.05127] Health
  (set `self.health` (- (`self.health`) Damage))
  (`self.Hit Reaction`)
  (`NiagaraFunctionLibrary.SpawnSystemAtLocation` "/Game/UI/NS_BloodSplatter.NS_BloodSplatter" (`SceneComponent.K2_GetComponentLocation` (`self.Blood Splatter Get Hit Pos`)) (struct) (1.0 1.0 1.0) true true "AutoRelease")
  (if (<= (`self.health`) 0.0)
    (`/Engine/EditorBlueprintResources/StandardMacros.DoOnce` false
      (:`Completed`
        (`PrimitiveComponent.SetSimulatePhysics` (`self.Mesh`) true)
        (bind _asbp_third_person_character (cast `/Game/ThirdPerson/Blueprints/BP_ThirdPersonCharacter` (`GameplayStatics.GetPlayerCharacter` 0)))
        (if (== (`/Game/ThirdPerson/Blueprints/BP_ThirdPersonCharacter.lockedTarget` _asbp_third_person_character) self)
          (`/Game/ThirdPerson/Blueprints/BP_ThirdPersonCharacter.Unlock Target` _asbp_third_person_character)
          (set `CharacterMovementComponent.MaxWalkSpeed` 0.0 (`self.CharacterMovement`))
          (`SceneComponent.SetVisibility` (`self.Health Bar`) false false))))))

(event `Hit Reaction`
  ;[0.05098 0.05098 0.05098] Impact Hit
)

(event `Sword Trace`
  ;[0.05098 0.05098 0.05098] Sword Attack Trace
  (bind _returnvalue (`KismetSystemLibrary.K2_SetTimerDelegate` (delegate `Trigger Sword Trace`) 0.001 true))
  (set `self.Sword Trigger Event` _returnvalue))

(event `Trigger Sword Trace`
  ;[0.05098 0.05098 0.05098] Sword Attack Trace
  (bind (_outhit _returnvalue) (`KismetSystemLibrary.SphereTraceSingle` :`Start` (`SceneComponent.K2_GetComponentLocation` (`self.Sword Top Socket`)) :`End` (`SceneComponent.K2_GetComponentLocation` (`self.Sword Bottom Socket`)) :`Radius` (`self.swordRadius`) :`TraceChannel` "TraceTypeQuery1" :`DrawTime` 0.1))
  (`NiagaraComponent.SetVariableFloat` (`self.NS_Trail`) "spawningrate" 90.0)
  (if _returnvalue
    (bind (_bblockinghit _binitialoverlap _time _distance _location _impactpoint _normal _impactnormal _physmat _hitactor) (`GameplayStatics.BreakHitResult` _outhit))
    (if (`self.ActorHasTag` _hitactor "Player")
      (`|ExecutionSequence`
        (:`then_0`
          (`/Engine/EditorBlueprintResources/StandardMacros.DoOnce` false :!label _label_3
            (:`Completed`
              (`KismetSystemLibrary.PrintString` "Enemy Hitted")
              (`GameplayStatics.ApplyDamage` _hitactor (`self.lightAttackDamage`))
              (`KismetSystemLibrary.Delay` 0.1)
              (goto _label_3 :!via `Reset`))))
        (:`then_1`
          (`/Engine/EditorBlueprintResources/StandardMacros.DoOnce` false :!label _label_4
            (:`Completed`
              (`NiagaraFunctionLibrary.SpawnSystemAtLocation` "/Game/UI/NS_BloodSplatter.NS_BloodSplatter" _impactpoint (struct) (1.0 1.0 1.0) true true "AutoRelease")
              (`GameplayStatics.PlaySoundAtLocation` "/Game/Audio/MS_Impact.MS_Impact" _impactpoint (struct) 1.0 1.0 0.0 null null null null)
              (`KismetSystemLibrary.Delay` 0.1)
              (goto _label_4 :!via `Reset`)))))
      (else
        (`/Engine/EditorBlueprintResources/StandardMacros.DoOnce` false :!label _label_5
          (:`Completed`
            (`GameplayStatics.PlaySoundAtLocation` "/Game/Audio/Boss_Hit_Stomp.Boss_Hit_Stomp" _impactpoint (struct) 0.4 1.0 0.0 "/Game/Audio/Footsteps/SA_Stomps.SA_Stomps" null null null)
            (`NiagaraFunctionLibrary.SpawnSystemAtLocation` "/Game/Niagara/NS_StompHit.NS_StompHit" _impactpoint (struct) (1.0 1.0 1.0) true true "AutoRelease")
            (`KismetSystemLibrary.Delay` 0.5)
            (goto _label_5 :!via `Reset`)))))))

(event `Stop Sword Trace`
  ;[0.05098 0.05098 0.05098] Sword Attack Trace
  (`KismetSystemLibrary.K2_ClearAndInvalidateTimerHandle` (`self.Sword Trigger Event`))
  (`NiagaraComponent.SetVariableFloat` (`self.NS_Trail`) "spawningrate" 0.0))

(fn `UserConstructionScript`)