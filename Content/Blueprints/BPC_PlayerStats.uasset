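; Player stats component for BP_ThirdPersonCharacter that tracks health, stamina, XP and level.
; It caches the owner a tick after BeginPlay, and most setters push values straight into the character's HUD stats widget.
; Decrease functions report depletion, while ResetHealth drains health to zero.
; Capped level-ups randomly scale the XP threshold and add 120% of current max health to the maximum without refilling current health.
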(event `self.ReceiveBeginPlay`
  (`KismetSystemLibrary.DelayUntilNextTick`)
  (bind _asbp_third_person_character (cast `/Game/ThirdPerson/Blueprints/BP_ThirdPersonCharacter` (`self.GetOwner`)))
  (set `self.Player Character BP` _asbp_third_person_character))

(fn `Decrease Health`
  (params (Damage :type "Float (double-precision)"))
  (returns (`Dead?` :type Boolean))
  (bind _hud_widget_stats (`/Game/ThirdPerson/Blueprints/BP_ThirdPersonCharacter.HUD Widget Stats` (`self.Player Character BP`)))
  (if (not (<= (`self.Current Health`) 0.0))
    (bind _output_get (set `self.Current Health` (- (`self.Current Health`) Damage)))
    (`ProgressBar.SetPercent` (`/Game/UI/Stats/Stats.HealthBar` _hud_widget_stats) (/ _output_get (`self.Max Health`)))
    (`TextBlock.SetText` (`/Game/UI/Stats/Stats.HealthText` _hud_widget_stats) (`KismetTextLibrary.Conv_DoubleToText` (`self.Current Health`) "HalfToEven"))
    (if (<= (`self.Current Health`) 0.0)
      _
      (else
        (return false))))
  (return true))

(fn `Decrease Stamina`
  (params (Stamina :type "Float (double-precision)"))
  (returns (`No Stamina Left` :type Boolean))
  (if (not (<= (`self.Current Stamina`) 0.0))
    (bind _output_get (set `self.Current Stamina` (- (`self.Current Stamina`) Stamina)))
    (`ProgressBar.SetPercent` (`/Game/UI/Stats/Stats.StaminaBar` (`/Game/ThirdPerson/Blueprints/BP_ThirdPersonCharacter.HUD Widget Stats` (`self.Player Character BP`))) (/ _output_get (`self.Max Stamina`)))
    (if (<= (`self.Current Stamina`) 0.0)
      _
      (else
        (return false))))
  (return true))

(fn `Get Current Health`
  (returns (`Current Health` :type "Float (double-precision)"))
  (return (`self.Current Health`)))

(fn `Increase Health`
  (params (`Added Health` :type "Float (double-precision)"))
  (bind _hud_widget_stats (`/Game/ThirdPerson/Blueprints/BP_ThirdPersonCharacter.HUD Widget Stats` (`self.Player Character BP`)))
  (set `self.Current Health` (+ (`self.Current Health`) `Added Health`))
  (if (> (`self.Current Health`) (`self.Max Health`))
    (set `self.Current Health` (`self.Max Health`)))
  (`self.Set Level and XP`)
  (`ProgressBar.SetPercent` (`/Game/UI/Stats/Stats.HealthBar` _hud_widget_stats) (/ (`self.Current Health`) (`self.Max Health`)))
  (`TextBlock.SetText` (`/Game/UI/Stats/Stats.HealthText` _hud_widget_stats) (`KismetTextLibrary.Conv_DoubleToText` (`self.Current Health`) "HalfToEven")))

(fn `Increase Level`
  (bind _hud_widget_stats (`/Game/ThirdPerson/Blueprints/BP_ThirdPersonCharacter.HUD Widget Stats` (`self.Player Character BP`)))
  (if (< (`self.Level`) 100)
    (set `self.Level` (+ (`self.Level`) 1))
    (set `self.XP` (- (`self.XP`) (`self.Max XP`)))
    (if (`KismetMathLibrary.RandomBool`)
      (set `self.Max XP` (* (`self.Max XP`) 1.05))
      (else
        (set `self.Max XP` (* (`self.Max XP`) 1.2))))
    (`ProgressBar.SetPercent` (`/Game/UI/Stats/Stats.XPBar` _hud_widget_stats) (/ (`self.XP`) (`self.Max XP`)))
    (`TextBlock.SetText` (`/Game/UI/Stats/Stats.XPText` _hud_widget_stats) (`KismetTextLibrary.Conv_DoubleToText` (`self.XP`) "HalfToEven"))
    (`TextBlock.SetText` (`/Game/UI/Stats/Stats.MaxXPText` _hud_widget_stats) (`KismetTextLibrary.Conv_DoubleToText` (`self.Max XP`) "HalfToEven"))
    (`TextBlock.SetText` (`/Game/UI/Stats/Stats.LevelText` _hud_widget_stats) "")
    (`self.Increase Max Health` (* (`self.Max Health`) 1.2))
    (else
      (set `self.XP` (`self.Max XP`)))))

(fn `Increase Max Health`
  (params (`Recovery Health` :type "Float (double-precision)"))
  (bind _hud_widget_stats (`/Game/ThirdPerson/Blueprints/BP_ThirdPersonCharacter.HUD Widget Stats` (`self.Player Character BP`)))
  (set `self.Max Health` (+ (`self.Max Health`) `Recovery Health`))
  (`ProgressBar.SetPercent` (`/Game/UI/Stats/Stats.HealthBar` _hud_widget_stats) (/ (`self.Current Health`) (`self.Max Health`)))
  (`TextBlock.SetText` (`/Game/UI/Stats/Stats.HealthText` _hud_widget_stats) (`KismetTextLibrary.Conv_DoubleToText` (`self.Current Health`) "HalfToEven")))

(fn `Increase Max Stamina`
  (params (`Recovery Stamina` :type "Float (double-precision)"))
  (set `self.Max Stamina` (+ (`self.Max Stamina`) `Recovery Stamina`))
  (`ProgressBar.SetPercent` (`/Game/UI/Stats/Stats.StaminaBar` (`/Game/ThirdPerson/Blueprints/BP_ThirdPersonCharacter.HUD Widget Stats` (`self.Player Character BP`))) (/ (`self.Current Stamina`) (`self.Max Stamina`))))

(fn `Increase Stamina`
  (params (`Added Stamina` :type "Float (double-precision)"))
  (set `self.Current Stamina` (+ (`self.Current Stamina`) `Added Stamina`))
  (if (> (`self.Current Stamina`) (`self.Max Stamina`))
    (set `self.Current Stamina` (`self.Max Stamina`)))
  (`ProgressBar.SetPercent` (`/Game/UI/Stats/Stats.StaminaBar` (`/Game/ThirdPerson/Blueprints/BP_ThirdPersonCharacter.HUD Widget Stats` (`self.Player Character BP`))) (/ (`self.Current Stamina`) (`self.Max Stamina`))))

(fn `Increase XP`
  (params (`Added XP` :type Integer))
  (set `self.XP` (+ (`self.XP`) (`KismetMathLibrary.Conv_IntToDouble` `Added XP`)))
  (if (>= (`self.XP`) (`self.Max XP`))
    (`self.Increase Level`)))

(fn `Reset Health`
  (`self.Decrease Health` (`self.Current Health`))
  (return))

(fn `Set Level and XP`
  (bind _hud_widget_stats (`/Game/ThirdPerson/Blueprints/BP_ThirdPersonCharacter.HUD Widget Stats` (`self.Player Character BP`)))
  (`ProgressBar.SetPercent` (`/Game/UI/Stats/Stats.XPBar` _hud_widget_stats) (/ (`self.XP`) (`self.Max XP`)))
  (`TextBlock.SetText` (`/Game/UI/Stats/Stats.XPText` _hud_widget_stats) (`KismetTextLibrary.Conv_DoubleToText` (`self.XP`) "HalfToEven"))
  (`TextBlock.SetText` (`/Game/UI/Stats/Stats.MaxXPText` _hud_widget_stats) (`KismetTextLibrary.Conv_DoubleToText` (`self.Max XP`) "HalfToEven"))
  (`TextBlock.SetText` (`/Game/UI/Stats/Stats.LevelText` _hud_widget_stats) (`KismetTextLibrary.Conv_IntToText` (`self.Level`))))

(fn `Stamina Info`
  (returns (Output :type Boolean))
  (if (> (`self.Current Stamina`) 0.0)
    (return true)
    (else
      (return false))))