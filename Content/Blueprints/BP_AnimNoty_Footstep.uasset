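; Footstep anim notify that plays step sounds at the mesh's world location.
; When the owner is a BP_Boss, it plays a stomp sound and a world camera shake centered on the mesh.
; For other owners, it picks the sound by current level name: brick footsteps in the Castle level, grass footsteps everywhere else.
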(fn `Received_Notify`
  (params (MeshComp :type "SkeletalMeshComponent Object Reference") (Animation :type "AnimSequenceBase Object Reference") (EventReference :type "AnimNotifyEventReference Structure (by ref)"))
  (returns (ReturnValue :type Boolean))
  (bind _returnvalue (`SceneComponent.K2_GetComponentLocation` MeshComp))
  (cast `/Game/Blueprints/BP_Boss` (`ActorComponent.GetOwner` MeshComp)
    (:`then`
      (`GameplayStatics.PlaySoundAtLocation` "/Game/Audio/Footsteps/MS_Stomp.MS_Stomp" _returnvalue (struct) 1.0 1.0 0.0 "/Game/Audio/Footsteps/SA_Stomps.SA_Stomps" null null null)
      (`GameplayStatics.PlayWorldCameraShake` "/Game/Blueprints/BP_BossCameraShakeStep.BP_BossCameraShakeStep_C" _returnvalue 2000.0))
    (:`CastFailed`
      (bind _returnvalue_2 (`GameplayStatics.GetCurrentLevelName` true))
      (if (not (`KismetStringLibrary.EqualEqual_StrStr` _returnvalue_2 "Castle"))
        (`GameplayStatics.PlaySoundAtLocation` "/Game/Audio/Footsteps/GrassFootstepsCue.GrassFootstepsCue" _returnvalue (struct) 1.0 1.0 0.0 "/Game/Audio/Footsteps/SA_Footsteps.SA_Footsteps" null null null)
        (else
          (`GameplayStatics.PlaySoundAtLocation` "/Game/Audio/Footsteps/Footstep_Brick.Footstep_Brick" _returnvalue (struct) 1.0 1.0 0.0 "/Game/Audio/Footsteps/SA_Footsteps.SA_Footsteps" null null null)))
      (return false))))